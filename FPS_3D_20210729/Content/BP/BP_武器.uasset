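; BP_武器 is a weapon Blueprint that handles automatic firing and magazine reloading.
; Holding the 開槍 (fire) input runs a Delay-paced loop that spawns an actor and a scaled-down particle effect at the weapon mesh, using up one bullet per shot.
; The loop stops on release or an empty magazine.
; The 換彈夾 (reload) event refills the magazine from total ammo, capped by what remains.
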(event Custom|換彈夾
  (Variables|Default|Set要補充的子彈數量 (- (Variables|Default|Get彈夾尺寸) (Variables|Default|Get目前子彈數量)))
  (if (>= (Variables|Default|Get子彈總數) (Variables|Default|Get要補充的子彈數量))
    _
    (else
      (Variables|Default|Set要補充的子彈數量 (Variables|Default|Get子彈總數))))
  (Variables|Default|Set目前子彈數量 (+ (Variables|Default|Get目前子彈數量) (Variables|Default|Get要補充的子彈數量)))
  (Variables|Default|Set子彈總數 (- (Variables|Default|Get子彈總數) (Variables|Default|Get要補充的子彈數量))))

(event Input|ActionEvents|InputAction開槍
  (params (Key :type Key%20Structure :default "None"))
  (bind _武器模型 (Variables|Default|Get武器模型))
  (:Pressed
    (Variables|Default|Set開槍中 true)
    (if (and (> (Variables|Default|Get目前子彈數量) 0) (Variables|Default|Get開槍中)) :!label _label
      (Game|SpawnActorfromClass "/Game/BP/BP_子彈.BP_子彈_C" (Transformation|GetSocketTransform (Variables|Default|Get武器模型) "子彈插槽" "RTS_World") "Undefined" 0 0)
      (Effects|SpawnEmitteratLocation "/Game/InfinityBladeEffects/Effects/FX_Combat_Base/Impact/P_Impact_Player_Fire_Strong.P_Impact_Player_Fire_Strong" (Transformation|GetSocketLocation _武器模型 "子彈插槽") (Transformation|GetSocketRotation _武器模型 "None") "0.080000,0.080000,0.080000")
      (Variables|Default|Set目前子彈數量 (- (Variables|Default|Get目前子彈數量) 1))
      (Utilities|FlowControl|Delay (Variables|Default|Get開槍間隔))
      (goto _label)))
  (:Released
    (Variables|Default|Set開槍中 false)))

(fn ConstructionScript)